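; BP_WorldGrid initializes the world at BeginPlay by spawning a tile grid, setting up villages and painting their species territories.
; It gathers every StaticMeshActor as a tile and every BP_Village, deriving each village's Species and Temperament from its array index before calling Setup.
; A brute-force distance check then swaps the second material slot of tiles near each village to its species material, so later villages win overlaps.
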(event `self.ReceiveBeginPlay`
  (`self.SpawnTileGrid`)
  (bind _outactors (`GameplayStatics.GetAllActorsOfClass` "/Script/Engine.StaticMeshActor"))
  (bind _output_get (set `self.AllTiles` _outactors))
  (`KismetSystemLibrary.PrintString` (`KismetStringLibrary.Concat_StrStr` "Tiles: " (`KismetStringLibrary.Conv_IntToString` (`KismetArrayLibrary.Array_Length` _output_get))))
  (bind _outactors_2 (`GameplayStatics.GetAllActorsOfClass` "/Game/Blueprints/BP_Village.BP_Village_C"))
  (bind _output_get_2 (set `self.Villages` _outactors_2))
  (`|ExecutionSequence`
    (:`then_0`
      (for (_array_element _array_index) _output_get_2
        (bind _returnvalue (`KismetArrayLibrary.Array_Length` _output_get_2))
        (set `/Game/Blueprints/BP_Village.Species` (cast `/Game/Blueprints/Data/ENUM/Villages/ENUM_Species` (`KismetMathLibrary.Conv_IntToByte` (mod _array_index _returnvalue))) _array_element)
        (set `/Game/Blueprints/BP_Village.Temperament` (cast `/Game/Blueprints/Data/ENUM/Villages/ENUM_Temperament` (`KismetMathLibrary.Conv_IntToByte` (mod _array_index 3))) _array_element)
        (`/Game/Blueprints/BP_Village.Setup` _array_element)))
    (:`then_1`
      (`KismetSystemLibrary.PrintString` (`KismetStringLibrary.Concat_StrStr` "Villages: " (`KismetStringLibrary.Conv_IntToString` _returnvalue)))
      (for _array_element_2 _output_get_2
        (for _array_element_3 (`self.AllTiles`)
          (if (<= (`KismetMathLibrary.Vector_Distance` (`self.K2_GetActorLocation` _array_element_3) (`self.K2_GetActorLocation` _array_element_2)) 1000.0)
            (switch `/Game/Blueprints/Data/ENUM/Villages/ENUM_Species` (`/Game/Blueprints/BP_Village.Species` _array_element_2)
              (:`NewEnumerator0`
                (bind _staticmeshcomponent (`StaticMeshActor.StaticMeshComponent` _array_element_3))
                (`PrimitiveComponent.SetMaterial` _staticmeshcomponent 1 "/Game/Materials/MI_Fishmen.MI_Fishmen"))
              (:`NewEnumerator1`
                (`PrimitiveComponent.SetMaterial` _staticmeshcomponent 1 "/Game/Materials/MI_Gnomes.MI_Gnomes"))
              (:`NewEnumerator2`
                (`PrimitiveComponent.SetMaterial` _staticmeshcomponent 1 "/Game/Materials/MI_Dragonborn.MI_Dragonborn"))
              (:`NewEnumerator3`
                (`PrimitiveComponent.SetMaterial` _staticmeshcomponent 1 "/Game/Materials/MI_Vampires.MI_Vampires"))
              (:`NewEnumerator4`
                (`PrimitiveComponent.SetMaterial` _staticmeshcomponent 1 "/Game/Materials/MI_Werewolves.MI_Werewolves")))))))))

(fn `UserConstructionScript`)