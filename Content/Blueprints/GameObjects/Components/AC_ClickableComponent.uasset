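; Actor component that makes its owner clickable, toggling its mesh material and showing village building info.
; On BeginPlay it binds click handlers and caches the owner's StaticMeshComponent.
; Clicks swap material slot 0, enable custom depth and, for BP_Village owners, add a new W_BuildingInfo widget.
; InPlacementMode destroys the component; the hover-end cleanup of outline and widget is never bound.
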(event `self.ReceiveBeginPlay`
  (bind _returnvalue (`self.GetOwner`))
  (bind _returnvalue_2 (`Actor.GetComponentByClass` _returnvalue "/Script/Engine.StaticMeshComponent"))
  (add `Actor.OnClicked` _returnvalue (delegate `OnMouseClicked`))
  (`/Engine/EditorBlueprintResources/StandardMacros.IsValid` _returnvalue_2
    (:`Is Valid`
      (set `self.StaticMeshRef` _returnvalue_2)
      (add `Actor.OnClicked` (`self.GetOwner`) (delegate `MouseOnClickedWidget`)))))

(event `MouseOnClickedWidget`
  (params (TouchedActor :type "Actor Object Reference") (ButtonPressed :type "Key Structure" :default "None"))
  (`PrimitiveComponent.SetRenderCustomDepth` (`self.StaticMeshRef`) true)
  (bind _asbp_village (cast `/Game/Blueprints/BP_Village` TouchedActor))
  (bind _returnvalue (`|CreateWidget` "/Game/Widgets/W_BuildingInfo.W_BuildingInfo_C" (`GameplayStatics.GetPlayerController` 0) _asbp_village))
  (`UserWidget.AddToViewport` _returnvalue 0))

(event `OnMouseHoverEnd`
  (params (TouchedActor :type "Actor Object Reference"))
  (`PrimitiveComponent.SetRenderCustomDepth` (`self.StaticMeshRef`) false)
  (`Widget.RemoveFromParent` (stale `MouseOnClickedWidget` _returnvalue)))

(event `OnMouseClicked`
  (params (TouchedActor :type "Actor Object Reference") (ButtonPressed :type "Key Structure" :default "None"))
  (bind _staticmeshref (`self.StaticMeshRef`))
  (set `self.isClicked` (not (`self.isClicked`)))
  (`/Engine/EditorBlueprintResources/StandardMacros.IsValid` (`self.StaticMeshRef`)
    (:`Is Valid`
      (if (`self.isClicked`)
        (`PrimitiveComponent.SetMaterial` _staticmeshref 0 "/Engine/VREditor/UI/KeyMaterial.KeyMaterial")
        (else
          (`PrimitiveComponent.SetMaterial` _staticmeshref 0 "/Engine/VREditor/UI/KeyDiskMaterial.KeyDiskMaterial"))))))

(event `InPlacementMode`
  (`self.K2_DestroyComponent`))