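; Actor component that makes its owner clickable and hoverable, apparently for buildings.
; On BeginPlay it binds the owner's click event, plus cursor-over events if a static mesh exists.
; Hover enables custom depth and shows a W_BuildingInfo widget for the ItemID, both undone on exit.
; Clicks toggle the mesh's first material between KeyMaterial and KeyDiskMaterial, and InPlacementMode destroys the component.
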(event `self.ReceiveBeginPlay`
  (bind _returnvalue (`self.GetOwner`))
  (bind _returnvalue_2 (`self.GetOwner`))
  (bind _returnvalue_3 (`Actor.GetComponentByClass` _returnvalue "/Script/Engine.StaticMeshComponent"))
  (add `Actor.OnClicked` _returnvalue (delegate `OnMouseClicked`))
  (`/Engine/EditorBlueprintResources/StandardMacros.IsValid` _returnvalue_3
    (:`Is Valid`
      (set `self.StaticMeshRef` _returnvalue_3)
      (add `Actor.OnBeginCursorOver` _returnvalue_2 (delegate `OnMouseHover`))
      (add `Actor.OnEndCursorOver` _returnvalue_2 (delegate `OnMouseHoverEnd`)))))

(event `OnMouseHoverEnd`
  (params (TouchedActor :type "Actor Object Reference"))
  (`PrimitiveComponent.SetRenderCustomDepth` (`self.StaticMeshRef`) false)
  (`Widget.RemoveFromParent` (stale `OnMouseHover` _returnvalue)))

(event `OnMouseHover`
  (params (TouchedActor :type "Actor Object Reference"))
  (`PrimitiveComponent.SetRenderCustomDepth` (`self.StaticMeshRef`) true)
  (bind _returnvalue (`|CreateWidget` "/Game/Widgets/W_BuildingInfo.W_BuildingInfo_C" (`GameplayStatics.GetPlayerController` 0) (`self.Item ID`)))
  (`UserWidget.AddToViewport` _returnvalue 0))

(event `OnMouseClicked`
  (params (TouchedActor :type "Actor Object Reference") (ButtonPressed :type "Key Structure" :default "None"))
  (bind _staticmeshref (`self.StaticMeshRef`))
  (set `self.isClicked` (not (`self.isClicked`)))
  (`/Engine/EditorBlueprintResources/StandardMacros.IsValid` (`self.StaticMeshRef`)
    (:`Is Valid`
      (if (`self.isClicked`)
        (`PrimitiveComponent.SetMaterial` _staticmeshref 0 "/Engine/VREditor/UI/KeyMaterial.KeyMaterial")
        (else
          (`PrimitiveComponent.SetMaterial` _staticmeshref 0 "/Engine/VREditor/UI/KeyDiskMaterial.KeyDiskMaterial"))))))

(event `InPlacementMode`
  (`self.K2_DestroyComponent`))