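; B_Build is a build-system Blueprint that shows a placement preview mesh where the player's camera is looking.
; A custom event caches the player pawn and its camera, and Tick runs the preview loop while InBuildMove is set.
; The loop line-traces 600 units forward with debug drawing, creates a demo box mesh on the pawn at the first hit, then moves it to each hit location with zero rotation.
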(event `CustomEvent`
  (bind _asbp_player_pawn (cast `/Game/Blueprints/BP_PlayerPawn` (`GameplayStatics.GetPlayerPawn` 0))
    (:`then`
      (set `self.PlayerPawn` _asbp_player_pawn)
      (set `self.Camera` (`/Game/Blueprints/BP_PlayerPawn.Camera` _asbp_player_pawn)))
    (:`CastFailed`
      (`KismetSystemLibrary.PrintString` "FAILEd"))))

(event `self.ReceiveTick`
  (params (DeltaSeconds :type "Float (single-precision)"))
  (if (`self.In Build Move?`)
    (`self.PreviewLoop`)))

(event `PreviewLoop`
  (bind (_returnvalue_location _returnvalue_rotation) (`KismetMathLibrary.BreakTransform` (`SceneComponent.K2_GetComponentToWorld` (`self.Camera`))))
  (bind (_outhit _returnvalue) (`KismetSystemLibrary.LineTraceSingle` :`Start` _returnvalue_location :`End` (+ _returnvalue_location (* (`KismetMathLibrary.GetForwardVector` _returnvalue_rotation) 600.0)) :`TraceChannel` "TraceTypeQuery1" :`DrawDebugType` "ForDuration"))
  (if _returnvalue
    (`|ExecutionSequence`
      (:`then_0`
        (`/Engine/EditorBlueprintResources/StandardMacros.DoOnce` false
          (:`Completed`
            (bind _returnvalue_2 (`|AddComponentByClass` (`self.PlayerPawn`) "/Script/Engine.StaticMeshComponent" false (`self.BuildPreviewTransform`)))
            (bind _output_get (set `self.PreviewMesh` _returnvalue_2))
            (`StaticMeshComponent.SetStaticMesh` _output_get "/Engine/Functions/Engine_MaterialFunctions02/ExampleContent/TextureBasedWPO/DemoBoxMesh.DemoBoxMesh"))))
      (:`then_1`
        (bind _output_get_2 (set `self.BuildPreviewTransform` (`KismetMathLibrary.MakeTransform` (`.Location` (`GameplayStatics.BreakHitResult` _outhit)))))
        (`SceneComponent.K2_SetWorldTransform` (`self.PreviewMesh`) _output_get_2 false false)))))