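; Game state for a ten-round portal-building economy game, tracking gold, rounds and village connections, and showing overlay and game-over widgets.
; CreatePortalConnection spawns paired portals beside two selected villages and deducts only the source portal's cost; DestroyPortalConnection is empty.
; NextRound converts a data-table-driven score of species needs, temperament and portal compatibility into gold.
; CalculateScore returns inside its loop, so only the first connection is scored.
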(event `self.ReceiveBeginPlay`
  (bind _returnvalue (`|CreateWidget` "/Game/Widgets/W_GameOverlay.W_GameOverlay_C" (`GameplayStatics.GetPlayerController` 0) self))
  (`UserWidget.AddToViewport` _returnvalue 0)
  (add `self.GameOver` (delegate `CreateGameOverWidget`))
  (bind _returnvalue_2 (`GameplayStatics.GetActorOfClass` "/Game/Blueprints/BP_WorldGrid.BP_WorldGrid_C"))
  (set `self.WorldGrid` _returnvalue_2))

(event `CreateGameOverWidget`
  (`self.GameOverState`)
  (`Widget.RemoveFromParent` (stale `self.ReceiveBeginPlay` _returnvalue)))

(fn `CalculateScore`
  (returns (Score :type Integer))
  (locals (CurrentPortalConnection :type "/Game/Blueprints/Data/FStruct_PortalConnection Structure"))
  (bind (_currentportalconnection_sourcevillage _currentportalconnection_destinationvillage) (break `/Game/Blueprints/Data/FStruct_PortalConnection` (`local.CurrentPortalConnection`)))
  (bind (_currentportalconnection_sourcevillage_2 _currentportalconnection_destinationvillage_2) (break `/Game/Blueprints/Data/FStruct_PortalConnection` (`local.CurrentPortalConnection`)))
  (bind (_currentportalconnection_sourcevillage_3 _currentportalconnection_destinationvillage_3) (break `/Game/Blueprints/Data/FStruct_PortalConnection` (`local.CurrentPortalConnection`)))
  (bind (_currentportalconnection_sourcevillage_4 _currentportalconnection_destinationvillage_4 _currentportalconnection_sourceportal _currentportalconnection_destinationportal) (break `/Game/Blueprints/Data/FStruct_PortalConnection` (`local.CurrentPortalConnection`)))
  (bind (_currentportalconnection_sourcevillage_5 _currentportalconnection_destinationvillage_5 _currentportalconnection_sourceportal_2) (break `/Game/Blueprints/Data/FStruct_PortalConnection` (`local.CurrentPortalConnection`)))
  (for _array_element (`self.PortalConnections`)
    (set `local.CurrentPortalConnection` _array_element)
    (bind _score (`self.GetVillageNeedFulfillmentScore` (`/Game/Blueprints/BP_Village.Species` _currentportalconnection_destinationvillage) (`/Game/Blueprints/BP_Village.Need` _currentportalconnection_sourcevillage)))
    (`self.PrintScoreName` "Village Need Fulfillment 1: " _score)
    (bind _score_2 (`self.GetVillageNeedFulfillmentScore` (`/Game/Blueprints/BP_Village.Species` _currentportalconnection_sourcevillage_2) (`/Game/Blueprints/BP_Village.Need` _currentportalconnection_destinationvillage_2)))
    (`self.PrintScoreName` "Village Need Fulfillment 2: " _score_2)
    (bind _score_3 (`self.GetTemperamentCompatibilityScore` (`/Game/Blueprints/BP_Village.Temperament` _currentportalconnection_sourcevillage_3) (`/Game/Blueprints/BP_Village.Temperament` _currentportalconnection_destinationvillage_3)))
    (`self.PrintScoreName` "Temperament Compatibility: " _score_3)
    (bind _score_4 (`self.GetPortalCompatibilityScore` (`/Game/Blueprints/BP_Village.Species` _currentportalconnection_sourcevillage_5) (`/Game/Blueprints/BP_Portal.Size` _currentportalconnection_sourceportal_2) (`/Game/Blueprints/BP_Portal.Type` _currentportalconnection_sourceportal_2)))
    (`self.PrintScoreName` "Portal Compatibility 1: " _score_4)
    (bind _score_5 (`self.GetPortalCompatibilityScore` (`/Game/Blueprints/BP_Village.Species` _currentportalconnection_destinationvillage_4) (`/Game/Blueprints/BP_Portal.Size` _currentportalconnection_destinationportal) (`/Game/Blueprints/BP_Portal.Type` _currentportalconnection_destinationportal)))
    (`self.PrintScoreName` "Portal Compatibility 2: " _score_5)
    (bind _returnvalue (+ _score_5 (+ _score_4 (+ (+ _score_2 _score) _score_3))))
    (`self.PrintScoreName` "Total Score: " _returnvalue)
    (return _returnvalue)))

(fn `CreatePortalConnection`
  (params (SourcePortalType :type "/Game/Blueprints/Data/ENUM/Portals/ENUM_PortalType Enum" :default "NewEnumerator0") (SourcePortalSize :type "/Game/Blueprints/Data/ENUM/Portals/ENUM_PortalSize Enum" :default "NewEnumerator0") (DestinationPortalType :type "/Game/Blueprints/Data/ENUM/Portals/ENUM_PortalType Enum" :default "NewEnumerator0") (DestinationPortalSize :type "/Game/Blueprints/Data/ENUM/Portals/ENUM_PortalSize Enum" :default "NewEnumerator0"))
  (bind _sourcevillage (`self.SourceVillage`))
  (bind _destinationvillage (`self.DestinationVillage`))
  (bind _tilesize (`WorldGrid.TileSize` (`self.WorldGrid`)))
  (bind _returnvalue (`|SpawnActorFromClass` "/Game/Blueprints/BP_Portal.BP_Portal_C" (`KismetMathLibrary.MakeTransform` (+ (`self.K2_GetActorLocation` _sourcevillage) (`KismetMathLibrary.MakeVector` (`KismetMathLibrary.Conv_IntToDouble` _tilesize) (`KismetMathLibrary.Conv_IntToDouble` _tilesize)))) "Undefined" "MultiplyWithRoot" null SourcePortalSize SourcePortalType null))
  (bind _returnvalue_2 (`|SpawnActorFromClass` "/Game/Blueprints/BP_Portal.BP_Portal_C" (`KismetMathLibrary.MakeTransform` (+ (`self.K2_GetActorLocation` _destinationvillage) (`KismetMathLibrary.MakeVector` (`KismetMathLibrary.Conv_IntToDouble` _tilesize) (`KismetMathLibrary.Conv_IntToDouble` _tilesize)))) "Undefined" "MultiplyWithRoot" null DestinationPortalSize DestinationPortalType null))
  (`KismetArrayLibrary.Array_Add` (`self.PortalConnections`) (make `/Game/Blueprints/Data/FStruct_PortalConnection` _sourcevillage _destinationvillage _returnvalue _returnvalue_2))
  (set `self.IsSettingSourceVillage` false)
  (set `self.IsSettingDestinationVillage` false)
  ;[1 1 1] Set to null
  (set `self.SourceVillage` null)
  (set `self.DestinationVillage` null)
  (bind _returnvalue_3 (`|GetDataTableRow` "/Game/Blueprints/Data/DT/DT_Portals.DT_Portals" (`KismetStringLibrary.Conv_StringToName` (`KismetStringLibrary.Concat_StrStr` (`|GetEnumeratorNameAsString` SourcePortalType) "_" (`|GetEnumeratorNameAsString` SourcePortalSize))))
    (:`then`
      (set `self.PlayerGold` (- (`self.PlayerGold`) (`.Cost_27_6C441EBF4275F12393EE8B9BE334565C` (break `/Game/Blueprints/Data/FStruct_PortalInfo` _returnvalue_3)))))))

(fn `DestroyPortalConnection`)

(fn `GameOverState`
  (bind _returnvalue (`|CreateWidget` "/Game/Widgets/W_GameOver.W_GameOver_C" null self))
  (`UserWidget.AddToViewport` _returnvalue 0)
  (`GameplayStatics.SetGamePaused` false))

(fn `GetPortalCompatibilityScore`
  (params (Species :type "/Game/Blueprints/Data/ENUM/Villages/ENUM_Species Enum" :default "NewEnumerator0") (PortalSize :type "/Game/Blueprints/Data/ENUM/Portals/ENUM_PortalSize Enum" :default "NewEnumerator0") (PortalType :type "/Game/Blueprints/Data/ENUM/Portals/ENUM_PortalType Enum" :default "NewEnumerator0"))
  (returns (Score :type Integer))
  (bind _returnvalue (`|GetDataTableRow` "/Game/Blueprints/Data/DT/DT_SpeciesPortalSizeCompatibility.DT_SpeciesPortalSizeCompatibility" (`KismetStringLibrary.Conv_StringToName` (`KismetStringLibrary.Concat_StrStr` (`|GetEnumeratorNameAsString` Species) "_" (`|GetEnumeratorNameAsString` PortalSize))))
    (:`then`
      (bind _returnvalue_2 (`|GetDataTableRow` "/Game/Blueprints/Data/DT/DT_SpeciesPortalTypeCompatibility.DT_SpeciesPortalTypeCompatibility" (`KismetStringLibrary.Conv_StringToName` (`KismetStringLibrary.Concat_StrStr` (`|GetEnumeratorNameAsString` Species) "_" (`|GetEnumeratorNameAsString` PortalType))))
        (:`then`
          (return (+ (`.Compatibility_8_56F3975E4470FDE42EE8269CBBB743C8` (break `/Game/Blueprints/Data/FStruct_SpeciesPortalTypeCompatibility` _returnvalue_2)) (`.Compatibility_13_2A1E5F6B47CED2BF94078C8165D943DD` (break `/Game/Blueprints/Data/FStruct_SpeciesPortalSizeCompatibility` _returnvalue)))))))))

(fn `GetTemperamentCompatibilityScore`
  (params (SourceTemperament :type "/Game/Blueprints/Data/ENUM/Villages/ENUM_Temperament Enum" :default "NewEnumerator0") (DestinationTemperament :type "/Game/Blueprints/Data/ENUM/Villages/ENUM_Temperament Enum" :default "NewEnumerator0"))
  (returns (Score :type Integer))
  (bind _returnvalue (`|GetDataTableRow` "/Game/Blueprints/Data/DT/DT_TemperamentCompatibility.DT_TemperamentCompatibility" (`KismetStringLibrary.Conv_StringToName` (`KismetStringLibrary.Concat_StrStr` (`|GetEnumeratorNameAsString` SourceTemperament) "_" (`|GetEnumeratorNameAsString` DestinationTemperament))))
    (:`then`
      (return (`.Compatibility_8_122637754F249A22135367AF88033282` (break `/Game/Blueprints/Data/FStruct_TemperamentCompatibility` _returnvalue))))
    (:`RowNotFound`
      (bind _returnvalue_2 (`|GetDataTableRow` "/Game/Blueprints/Data/DT/DT_TemperamentCompatibility.DT_TemperamentCompatibility" (`KismetStringLibrary.Conv_StringToName` (`KismetStringLibrary.Concat_StrStr` (`|GetEnumeratorNameAsString` DestinationTemperament) "_" (`|GetEnumeratorNameAsString` SourceTemperament))))
        (:`then`
          (return (`.Compatibility_8_122637754F249A22135367AF88033282` (break `/Game/Blueprints/Data/FStruct_TemperamentCompatibility` _returnvalue_2))))))))

(fn `GetVillageNeedFulfillmentScore`
  (params (Species :type "/Game/Blueprints/Data/ENUM/Villages/ENUM_Species Enum" :default "NewEnumerator0") (Need :type "/Game/Blueprints/Data/ENUM/Villages/ENUM_Need Enum" :default "NewEnumerator0"))
  (returns (Score :type Integer))
  (bind _returnvalue (`KismetStringLibrary.Conv_StringToName` (`KismetStringLibrary.Concat_StrStr` (`KismetStringLibrary.Replace` (`|GetEnumeratorNameAsString` Need) " " "" "CaseSensitive") "_" (`|GetEnumeratorNameAsString` Species))))
  (bind _returnvalue_2 (`|GetDataTableRow` "/Game/Blueprints/Data/DT/DT_SpeciesNeedFulfillment.DT_SpeciesNeedFulfillment" _returnvalue)
    (:`then`
      (return (`.Fulfill_24_3EDF27314D9C12A34E3C00A9A4E70F02` (break `/Game/Blueprints/Data/FStruct_SpeciesNeedFulfillment` _returnvalue_2))))
    (:`RowNotFound`
      (`KismetSystemLibrary.PrintString` (`KismetStringLibrary.Concat_StrStr` "Did not find: " (`KismetStringLibrary.Conv_NameToString` _returnvalue))))))

(fn `NextRound`
  (`/Engine/EditorBlueprintResources/StandardMacros.IncrementInt` (`self.Round`)
    (:`  `
      (set `self.CurrentRound` (`self.Round`))
      (`self.RewardRoundGold`)
      (if (> (`self.CurrentRound`) 10)
        (`self.GameOver`)))))

(fn `PrintScoreName`
  (params (Name :type String) (Score :type Integer))
  (`KismetSystemLibrary.PrintString` (`KismetStringLibrary.Concat_StrStr` Name (`KismetStringLibrary.Conv_IntToString` Score))))

(fn `RewardRoundGold`
  (bind _score (`self.CalculateScore`))
  (bind _gold (`self.ScoreToGold` _score))
  (set `self.PlayerGold` (+ (`self.PlayerGold`) _gold)))

(fn `ScoreToGold`
  (params (Score :type Integer))
  (returns (Gold :type Integer))
  (bind _score (`local.Score`))
  (bind _score_2 (`local.Score`))
  (bind _score_3 (`local.Score`))
  (bind _score_4 (`local.Score`))
  (if (and (>= Score 8) (< Score 16))
    (return 1)
    (elif (and (>= _score 16) (< _score 21))
      (return 2)
      (elif (and (>= _score_2 21) (< _score_2 26))
        (return 3)
        (elif (and (>= _score_3 26) (< _score_3 31))
          (return 4)
          (elif (and (>= _score_4 31) (< _score_4 36))
            (return 5)
            (elif (>= (`local.Score`) 36)
              (return 6))))))))

(fn `UserConstructionScript`)