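; Player pawn for a building-placement game, with cursor-driven placement, planar movement and clamped orthographic camera zoom.
; Placement mode starts on BeginPlay, spawning a preview actor with a ploppable component that follows a mouse line trace each tick.
; Clicking spawns a building at the preview's transform when its ploppable component reports a valid spot.
; The build input separately flip-flops the InBuildMove flag, leaving placement mode on.
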(event `self.ReceiveBeginPlay`
  (bind _asplayer_controller (cast `PlayerController` (`self.GetController`)))
  (bind _output_get (set `self.PlayerController` _asplayer_controller))
  (message `EnhancedInputSubsystemInterface.AddMappingContext` (pcsubsystem `EnhancedInputLocalPlayerSubsystem` _output_get) "/Game/Input/InputMappingContext.InputMappingContext" 0 (struct))
  (set `PlayerController.bShowMouseCursor` true (`self.PlayerController`))
  (`self.SetPlacementModeEnabled` true))

(event `EnhancedInput|/Game/Input/IA_Move`
  (params (ActionValue :type "Vector2D Structure") (ElapsedSeconds :type "Float (double-precision)") (TriggeredSeconds :type "Float (double-precision)") (InputAction :type "InputAction Object Reference" :default "/Game/Input/IA_Move.IA_Move"))
  (bind (_returnvalue_x _returnvalue_y) (`KismetMathLibrary.BreakVector2D` (* ActionValue (`self.MovementSpeed`))))
  (:`Triggered`
    (`PawnMovementComponent.AddInputVector` (`self.FloatingPawnMovement`) (`KismetMathLibrary.MakeVector` _returnvalue_x _returnvalue_y) false)))

(event `EnhancedInput|/Game/Input/IA_Zoom`
  (params (ActionValue :type "Float (double-precision)") (ElapsedSeconds :type "Float (double-precision)") (TriggeredSeconds :type "Float (double-precision)") (InputAction :type "InputAction Object Reference" :default "/Game/Input/IA_Zoom.IA_Zoom"))
  (:`Triggered`
    (bind _result (`/Engine/EditorBlueprintResources/StandardMacros.NegateFloat` ActionValue)
      (:`  `
        (`CameraComponent.SetOrthoWidth` (`self.Camera`) (`KismetMathLibrary.FMax` (`KismetMathLibrary.FMin` (+ (* _result (`self.ZoomSpeed`)) (`CameraComponent.OrthoWidth` (`self.Camera`))) (`self.MaxZoom`)) (`self.MinZoom`)))))))

(event `EnhancedInput|/Game/Input/IA_Build`
  (params (ActionValue :type Boolean) (ElapsedSeconds :type "Float (double-precision)") (TriggeredSeconds :type "Float (double-precision)") (InputAction :type "InputAction Object Reference" :default "/Game/Input/IA_Build.IA_Build"))
  (bind _b_build (`self.B_Build`))
  (:`Started`
    (`/Engine/EditorBlueprintResources/StandardMacros.FlipFlop`
      (:`A`
        (set `/Game/Blueprints/BuildSystem/B_Build.In Build Move?` true _b_build))
      (:`B`
        (set `/Game/Blueprints/BuildSystem/B_Build.In Build Move?` false _b_build)))))

(event `self.ReceiveTick`
  (params (DeltaSeconds :type "Float (single-precision)"))
  (if (`self.PlacementModeEnabled`)
    (`self.UpdatePlacement`)))

(event `EnhancedInput|/Game/Input/IA_Click`
  (params (ActionValue :type Boolean) (ElapsedSeconds :type "Float (double-precision)") (TriggeredSeconds :type "Float (double-precision)") (InputAction :type "InputAction Object Reference" :default "/Game/Input/IA_Click.IA_Click"))
  (:`Started`
    (if (`self.PlacementModeEnabled`)
      (`self.SpawnBuilding`))))

(fn `SetPlacementModeEnabled`
  (params (isEnabled :type Boolean))
  (bind _placeableactor (`self.PlaceableActor`))
  (if (== isEnabled (`self.PlacementModeEnabled`))
    (return)
    (else
      (bind _output_get (set `self.PlacementModeEnabled` isEnabled))
      (if _output_get
        (bind _returnvalue (`|SpawnActorFromClass` (`self.PlaceableActorType`) (`KismetMathLibrary.MakeTransform` (0.0 0.0 -100000.0)) "Undefined" "MultiplyWithRoot" null null))
        (bind _output_get_2 (set `self.PlaceableActor` _returnvalue))
        (bind _returnvalue_2 (`self.GetComponentByClass` _output_get_2 "/Game/Blueprints/GameObjects/Components/AC_ClickableCompoenet.AC_ClickableCompoenet_C"))
        (`/Engine/EditorBlueprintResources/StandardMacros.IsValid` _returnvalue_2
          (:`Is Valid`
            (`/Game/Blueprints/GameObjects/Components/AC_ClickableCompoenet.InPlacementMode` _returnvalue_2))
          (:`Is Not Valid`
            _))
        (`AddComponent|NODE_AddAC_PloppableComponent-0` :`self` (`self.PlaceableActor`))
        (else
          (`/Engine/EditorBlueprintResources/StandardMacros.IsValid` _placeableactor
            (:`Is Valid`
              (`self.K2_DestroyActor` _placeableactor))))))))

(fn `SpawnBuilding`
  (bind _returnvalue (`self.GetComponentByClass` (`self.PlaceableActor`) "/Game/Blueprints/GameObjects/Components/AC_PloppableComponent.AC_PloppableComponent_C"))
  (`/Engine/EditorBlueprintResources/StandardMacros.IsValid` _returnvalue
    (:`Is Valid`
      (if (`/Game/Blueprints/GameObjects/Components/AC_PloppableComponent.isPlacableValid` _returnvalue)
        (`|SpawnActorFromClass` (`self.PlaceableActorType`) (`self.GetTransform` (`self.PlaceableActor`)) "AlwaysSpawn" "MultiplyWithRoot" null null)))))

(fn `UpdatePlacement`
  (bind (_worldlocation _worlddirection) (`PlayerController.DeprojectMousePositionToWorld` (`GameplayStatics.GetPlayerController` 0)))
  (bind _outhit (`KismetSystemLibrary.LineTraceSingle` _worldlocation (+ _worldlocation (* _worlddirection 10000.0)) "TraceTypeQuery3"))
  (bind (_bblockinghit _binitialoverlap _time _distance _location) (`GameplayStatics.BreakHitResult` _outhit))
  (if _bblockinghit
    (`self.K2_SetActorLocation` (`self.PlaceableActor`) _location false false)))

(fn `UserConstructionScript`)