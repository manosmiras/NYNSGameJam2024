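; BP_Village is a village Blueprint that rolls a random Species, Temperament and Need for itself at BeginPlay.
; A sequence converts a random integer to the matching enum for each trait and stores it in a variable.
; A disconnected node, which never runs, would set the clickable component's ItemID to a random numbered "Village_" name.
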(event `self.ReceiveBeginPlay`
  (`|ExecutionSequence`
    (:`then_0`
      (set `self.Species` (cast `/Game/Blueprints/Data/ENUM/Villages/ENUM_Species` (`KismetMathLibrary.Conv_IntToByte` (`KismetMathLibrary.RandomIntegerInRange` 0 4)))))
    (:`then_1`
      (set `self.Temperament` (cast `/Game/Blueprints/Data/ENUM/Villages/ENUM_Temperament` (`KismetMathLibrary.Conv_IntToByte` (`KismetMathLibrary.RandomIntegerInRange` 0 2)))))
    (:`then_2`
      (set `self.Need` (cast `/Game/Blueprints/Data/ENUM/Villages/ENUM_Need` (`KismetMathLibrary.Conv_IntToByte` (`KismetMathLibrary.RandomIntegerInRange` 0 4)))))))

(fn `UserConstructionScript`)